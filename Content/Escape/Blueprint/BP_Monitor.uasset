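; BP_Monitor is an escape-game monitor with a keypad widget for entering a code to unlock it.
; On BeginPlay it enables input, takes the escape pawn's left and right widget interaction components, and binds to the password UI's code-entry event.
; Trigger presses act as pointer clicks on the keypad.
; CheckCode clears the entry and, on a match, unlocks, disables input and calls Spawn1 on BP_Spawner.
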(event EventBeginPlay
  (Utilities|FlowControl|Sequence
    (:then_0
      (CallFunction|EnableInputKeypad))
    (:then_1
      (bind _aspassword_ui (Utilities|Casting|CastToPassword_UI (UserInterface|GetUserWidgetObject (Variables|Default|GetKeyPad))))
      (bind _output_get (Variables|Default|SetPassword%20UI _aspassword_ui))
      (EventDispatchers|BindEventtoCodeEnter _output_get (EventDispatchers|CreateEvent :!event CheckCode)))))

(event Input|ActionEvents|InputActionTriggerLeft
  (params (Key :type Key%20Structure :default "None"))
  (bind _widget_interaction_left (Variables|Default|GetWidget%20Interaction%20Left))
  ;[0.03434 0.03434 0.03434] Menu Input Left/Right
  (:Pressed
    (Class|WidgetInteractionComponent|PressPointerKey _widget_interaction_left "LeftMouseButton"))
  (:Released
    (Class|WidgetInteractionComponent|ReleasePointerKey _widget_interaction_left "LeftMouseButton")))

(event Input|ActionEvents|InputActionTriggerRight
  (params (Key :type Key%20Structure :default "None"))
  (bind _widget_interaction_right (Variables|Default|GetWidget%20Interaction%20Right))
  ;[0.03434 0.03434 0.03434] Menu Input Left/Right
  (:Pressed
    (Class|WidgetInteractionComponent|PressPointerKey _widget_interaction_right "LeftMouseButton"))
  (:Released
    (Class|WidgetInteractionComponent|ReleasePointerKey _widget_interaction_right "LeftMouseButton")))

(fn ConstructionScript)

(fn CheckCode
  (params (Code :type String) (PasswordUI :type Password%20UI%20Object%20Reference))
  (if (Utilities|Enum|Equal(Enum) Code (Variables|Default|GetCode))
    (Variables|Default|SetIsLock false)
    (Variables|/Game/Escape/Widget/Password_UI.Password_UI_C|SetCurruntCode (Variables|Default|GetPassword%20UI) "")
    (Input|DisableInput (Game|GetPlayerController 0))
    (bind _returnvalue (Actor|GetActorOfClass "/Game/Escape/Blueprint/BP_Spawner.BP_Spawner_C"))
    (Default|Spawn1 _returnvalue)
    (else
      (Variables|/Game/Escape/Widget/Password_UI.Password_UI_C|SetCurruntCode (Variables|Default|GetPassword%20UI) ""))))

(fn EnableInputKeypad
  (Input|EnableInput (Game|GetPlayerController 0))
  (bind _asbp_escape_pawn (Utilities|Casting|CastToBP_EscapePawn (Game|Player|GetPlayerPawn 0)))
  (Variables|Default|SetWidget%20Interaction%20Left (Variables|/Game/Escape/BP_EscapePawn.BP_EscapePawn_C|GetWidgetInteractionLeft _asbp_escape_pawn))
  (Variables|Default|SetWidget%20Interaction%20Right (Variables|/Game/Escape/BP_EscapePawn.BP_EscapePawn_C|GetWidgetInteractionRight _asbp_escape_pawn)))