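; Spawner actor for an escape game that places puzzle props when its Spawn1 or Spawn2 event fires.
; Spawn1 creates the first glass board and a hint, then enables player input on the small safe door.
; Spawn2 creates the second glass board and a door lock.
; Boards appear at the spawner's location, while the hint and lock use hardcoded world positions.
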(event EventSpawn1
  (CallFunction|SpawnBoard1)
  (CallFunction|InputSafeSmall))

(event EventSpawn2
  (CallFunction|SpawnBoard2))

(fn ConstructionScript)

(fn SpawnBoard2
  (Utilities|FlowControl|Sequence
    (:then_0
      (Game|SpawnActorfromClass "/Game/Escape/Blueprint/BP_GlassBoard2.BP_GlassBoard2_C" (Math|Transform|MakeTransform (.location (Transformation|GetActorTransform)) "0.0,180.000000,0.0" "1,1,1") "Undefined" 0 0))
    (:then_1
      (Game|SpawnActorfromClass "/Game/Escape/Blueprint/BP_DoorLock.BP_DoorLock_C" (Math|Transform|MakeTransform (Math|Vector|MakeVector 1.45e+03 4e+01 65.0) (Math|Rotator|MakeRotator 0.0 0.0 1.8e+02) "2.500000,2.500000,2.500000") "Undefined" 0 0))))

(fn SpawnBoard1
  (Utilities|FlowControl|Sequence
    (:then_0
      (Game|SpawnActorfromClass "/Game/Escape/Blueprint/BP_GlassBoard.BP_GlassBoard_C" (Math|Transform|MakeTransform (.location (Transformation|GetActorTransform)) "0.0,180.000000,0.0" "1,1,1") "Undefined" 0 0))
    (:then_1
      (Game|SpawnActorfromClass "/Game/Escape/Blueprint/BP_Hint1.BP_Hint1_C" (Math|Transform|MakeTransform (Math|Vector|MakeVector 1.35e+03 -4e+02 7e+01) "0, 0, 0" "1,1,1") "Undefined" 0 0))))

(fn InputSafeSmall
  (bind _returnvalue (Actor|GetActorOfClass "/Game/Escape/Blueprint/BP_SafesmallDoor.BP_SafesmallDoor_C"))
  (Input|EnableInput _returnvalue (Game|GetPlayerController 0))
  (bind _asbp_escape_pawn (Utilities|Casting|CastToBP_EscapePawn (Game|Player|GetPlayerPawn 0)))
  (Variables|Default|SetWidget%20Interaction%20Left (Variables|/Game/Escape/BP_EscapePawn.BP_EscapePawn_C|GetWidgetInteractionLeft _asbp_escape_pawn))
  (Variables|Default|SetWidget%20Interaction%20Right (Variables|/Game/Escape/BP_EscapePawn.BP_EscapePawn_C|GetWidgetInteractionRight _asbp_escape_pawn)))