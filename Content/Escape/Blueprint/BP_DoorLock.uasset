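; BP_DoorLock is a keypad door lock for an escape game, built on a DoorKeyPad widget in its DoorKey component.
; On BeginPlay it enables player input, caches the escape pawn's left and right widget interaction components, and binds to the keypad's code-enter event.
; CheckCode clears the typed code after each check, and on a match also unlocks the door and disables input.
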(event EventBeginPlay
  (Utilities|FlowControl|Sequence
    (:then_0
      (CallFunction|InputDoorLockKey))
    (:then_1
      (bind _asdoor_key_pad (Utilities|Casting|CastToDoorKeyPad (UserInterface|GetUserWidgetObject (Variables|Default|GetDoorKey))))
      (bind _output_get (Variables|Default|SetDoorKeyPad _asdoor_key_pad))
      (EventDispatchers|BindEventtoCodeEnter _output_get (EventDispatchers|CreateEvent :!event CheckCode)))))

(fn ConstructionScript)

(fn InputDoorLockKey
  (Input|EnableInput (Game|GetPlayerController 0))
  (bind _asbp_escape_pawn (Utilities|Casting|CastToBP_EscapePawn (Game|Player|GetPlayerPawn 0)))
  (Variables|Default|SetWidget%20Interaction%20Left (Variables|/Game/Escape/BP_EscapePawn.BP_EscapePawn_C|GetWidgetInteractionLeft _asbp_escape_pawn))
  (Variables|Default|SetWidget%20Interaction%20Right (Variables|/Game/Escape/BP_EscapePawn.BP_EscapePawn_C|GetWidgetInteractionRight _asbp_escape_pawn)))

(fn CheckCode
  (params (Code :type String) (PasswordUI :type Door%20Key%20Pad%20Object%20Reference))
  (if (Utilities|Enum|Equal(Enum) Code (Variables|Default|GetCode))
    (Variables|Default|SetIsLock false)
    (Variables|/Game/Escape/Widget/DoorKeyPad.DoorKeyPad_C|SetCurruntCode (Variables|Default|GetDoorKeyPad) "")
    (Input|DisableInput (Game|GetPlayerController 0))
    (else
      (Variables|/Game/Escape/Widget/DoorKeyPad.DoorKeyPad_C|SetCurruntCode (Variables|Default|GetDoorKeyPad) ""))))