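; BP_RoomEnter is an escape-room actor that lets the player's motion controllers click widget menus.
; On BeginPlay it enables player input on itself and caches the left and right WidgetInteraction components from BP_EscapePawn.
; Each trigger's press and release is forwarded to the matching component as a left mouse button press or release, simulating pointer clicks on UI.
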(event EventBeginPlay
  (Input|EnableInput (Game|GetPlayerController 0))
  (bind _asbp_escape_pawn (Utilities|Casting|CastToBP_EscapePawn (Game|Player|GetPlayerPawn 0)))
  (Variables|Default|SetWidget%20Interaction%20Left (Variables|/Game/Escape/BP_EscapePawn.BP_EscapePawn_C|GetWidgetInteractionLeft _asbp_escape_pawn))
  (Variables|Default|SetWidget%20Interaction%20Right (Variables|/Game/Escape/BP_EscapePawn.BP_EscapePawn_C|GetWidgetInteractionRight _asbp_escape_pawn)))

(event Input|ActionEvents|InputActionTriggerLeft
  (params (Key :type Key%20Structure :default "None"))
  (bind _widget_interaction_left (Variables|Default|GetWidget%20Interaction%20Left))
  ;[0.03434 0.03434 0.03434] Menu Input Left
  (:Pressed
    (Class|WidgetInteractionComponent|PressPointerKey _widget_interaction_left "LeftMouseButton"))
  (:Released
    (Class|WidgetInteractionComponent|ReleasePointerKey _widget_interaction_left "LeftMouseButton")))

(event Input|ActionEvents|InputActionTriggerRight
  (params (Key :type Key%20Structure :default "None"))
  (bind _widget_interaction_right (Variables|Default|GetWidget%20Interaction%20Right))
  ;[0.03434 0.03434 0.03434] Menu Input Right
  (:Pressed
    (Class|WidgetInteractionComponent|PressPointerKey _widget_interaction_right "LeftMouseButton"))
  (:Released
    (Class|WidgetInteractionComponent|ReleasePointerKey _widget_interaction_right "LeftMouseButton")))

(fn ConstructionScript)